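; BP_Blood_Drops leaves blood decals where its Niagara blood effect reports particles.
; On BeginPlay it passes itself to the Niagara system as a user object to receive exported particle data.
; Each particle spawns a decal at its position, facing against its velocity, which fades out after a delay with destroy-owner enabled.
; The random size blend has a zero range, so decals always spawn at one-fifth of DecalSize.
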(event EventParticleData
  (params (Data :type Array%20of%20Basic%20Particle%20Data%20Structures) (NiagaraSystem :type Niagara%20System%20Object%20Reference) (SimulationPositionOffset :type Vector%20%28by%20ref%29 :default "0, 0, 0"))
  (bind _decalsize (Variables|Default|GetDecalSize))
  ;[1 1 1] Kanın yavaş yavaş fade out olması
  (for _array_element Data
    (bind _returnvalue (Rendering|Decal|SpawnDecalatLocation "/Game/VFX/VFX_Blood/M_Blood_Decal.M_Blood_Decal" (Math|Conversions|ToVector(Float) (Math|Float|Lerp (* _decalsize 0.2) _decalsize (Math|Random|RandomFloatinRange 0.0 0.0))) (.Position (Utilities|Struct|BreakBasicParticleData _array_element)) (Math|Conversions|RotationFromXVector (* (.Velocity (Utilities|Struct|BreakBasicParticleData _array_element)) -1.0)) 0.0))
    (Rendering|Components|Decal|SetFadeOut _returnvalue 3.0 5.0 true)))

(event EventBeginPlay
  (Class|NiagaraComponent|SetVariableObject (Variables|Default|GetNS_Blood_Effect) "BP_Blood" self))

(fn ConstructionScript)